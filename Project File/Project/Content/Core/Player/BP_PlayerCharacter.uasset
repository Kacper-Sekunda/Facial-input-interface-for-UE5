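; BP_PlayerCharacter is the player character, with a blink effect triggered by pressing Space Bar.
; The PlayerBlink event lazily creates a WBP_Blink widget, adds it to the viewport and caches it for reuse.
; Each blink plays that widget's FadeInOut animation.
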(event Custom|PlayerBlink
  (if (Utilities|IsValid (Variables|Default|GetWBP_Blink))
    _
    (else
      (bind _returnvalue (UserInterface|CreateWidget "/Game/Art/Widgets/WBP_Blink.WBP_Blink_C"))
      (UserInterface|Viewport|AddtoViewport _returnvalue 0)
      (Variables|Default|SetWBP_Blink _returnvalue)))
  (UserInterface|Animation|PlayAnimation (Variables|Default|GetWBP_Blink) (Variables|/Game/Art/Widgets/WBP_Blink.WBP_Blink_C|GetFadeInOut (Variables|Default|GetWBP_Blink)) 0.0 1 "Forward" 1.0 false))

(event EventBeginPlay)

(event Input|KeyboardEvents|SpaceBar
  (params (Key :type Key%20Structure :default "None"))
  (:Pressed
    (CallFunction|PlayerBlink)))

(fn ConstructionScript)