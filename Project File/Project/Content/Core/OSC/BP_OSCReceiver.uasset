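; BP_OSCReceiver receives face-tracking events over OSC and passes blinks on to the player character.
; On BeginPlay it starts a local OSC server, binds a message handler and caches the BP_PlayerCharacter reference.
; The handler switches on the message address path: blink calls PlayerBlink on the character, while mouth-open and loading-status messages only print debug strings.
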(event Custom|HandleOSCMessage
  (params (Message :type OSC%20Message%20Structure%20%28by%20ref%29) (IPAddress :type String) (Port :type Integer))
  (bind _returnvalue (Class|OSCManager|GetOSCMessageAddress Message))
  (bind _returnvalue_2 (Class|OSCManager|GetOSCAddressFullPath _returnvalue))
  (switch string _returnvalue_2
    (:/face/blink
      (Development|PrintString "Blinked")
      (Default|PlayerBlink (stale EventBeginPlay _output_get_2)))
    (:/face/mouth_open
      (Development|PrintString "Opened_Mouth"))
    (:/face/loaded
      (Development|PrintString "Loaded"))
    (:/face/loading
      (Development|PrintString "Loading"))))

(event EventBeginPlay
  (bind _returnvalue (Class|OSCManager|CreateOSCServer "127.0.0.1" 8000 false true "" 0))
  (bind _output_get (Variables|Default|SetOSCServerRef _returnvalue))
  (EventDispatchers|BindEventtoOnOscMessageReceived _output_get (delegate Custom|HandleOSCMessage))
  (bind _asbp_player_character (Utilities|Casting|CastToBP_PlayerCharacter (Game|GetPlayerCharacter 0)))
  (bind _output_get_2 (Variables|Default|SetAs%20BP%20Player%20Character _asbp_player_character)))

(fn ConstructionScript)